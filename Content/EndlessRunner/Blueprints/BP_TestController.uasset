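; BP_TestController is the player controller for the endless runner, turning input into character actions and setting up the HUD.
; On BeginPlay it caches the possessed BP_TestCharacter, printing a warning if the cast fails, then creates UMG_HUD, adds it to the viewport and keeps a reference.
; Left, Right and Jump input actions forward to that character's SwitchLane and DoJump functions.
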(event EventBeginPlay
  (Utilities|FlowControl|Sequence
    (:then_0
      (bind _asbp_test_character (Utilities|Casting|CastToBP_TestCharacter (Pawn|GetControlledPawn))
        (:then
          (Variables|Default|SetMyPawn _asbp_test_character))
        (:CastFailed
          (Development|PrintString "No pawn detected."))))
    (:then_1
      (bind _returnvalue (UserInterface|CreateWidget "/Game/EndlessRunner/UMG/UMG_HUD.UMG_HUD_C" self))
      (UserInterface|Viewport|AddtoViewport _returnvalue 0)
      (Variables|Default|SetMyCustomHUD _returnvalue))))

(event Input|ActionEvents|InputActionLeft
  (params (Key :type Key%20Structure :default "None"))
  (:Pressed
    (Default|SwitchLane (Variables|Default|GetMyPawn) false)))

(event Input|ActionEvents|InputActionRight
  (params (Key :type Key%20Structure :default "None"))
  (:Pressed
    (Default|SwitchLane (Variables|Default|GetMyPawn) true)))

(event Input|ActionEvents|InputActionJump
  (params (Key :type Key%20Structure :default "None"))
  (:Pressed
    (Default|DoJump (Variables|Default|GetMyPawn))))

(fn ConstructionScript)