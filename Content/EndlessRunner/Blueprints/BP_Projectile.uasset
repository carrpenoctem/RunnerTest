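; BP_Projectile is an endless runner projectile that kills the player on overlap.
; The construction script feeds a normalized Velocity into ProjectileMovement and sets its initial speed.
; Overlapping any actor other than its owner spawns an explosion and destroys it, first calling DoDie on BP_TestCharacter if that actor is the player.
; A delay started on BeginPlay destroys it after a fixed lifetime, without an explosion.
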(event EventBeginPlay
  (Utilities|FlowControl|Delay 5.0)
  (Actor|DestroyActor))

(event Collision|EventActorBeginOverlap
  (params (OtherActor :type Actor%20Object%20Reference))
  (bind _returnvalue (Game|GetPlayerCharacter 0))
  (if (!= OtherActor (Components|GetOwner))
    (if (== OtherActor _returnvalue)
      (Default|DoDie (.AsBP%20Test%20Character (Utilities|Casting|CastToBP_TestCharacter _returnvalue))))
    (Effects|SpawnEmitteratLocation "/Game/StarterContent/Particles/P_Explosion.P_Explosion" (Transformation|GetActorLocation))
    (Actor|DestroyActor)))

(event EventTick
  (params (DeltaSeconds :type Float%20%28single-precision%29)))

(fn ConstructionScript
  (bind _projectilemovement (Variables|Default|GetProjectileMovement))
  (Variables|/Script/Engine.MovementComponent|SetVelocity _projectilemovement (Math|Vector|Normalize (Variables|Default|GetVelocity)))
  (Variables|/Script/Engine.ProjectileMovementComponent|SetInitialSpeed _projectilemovement 8e+02))