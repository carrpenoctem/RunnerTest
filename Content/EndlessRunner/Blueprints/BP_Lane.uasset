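; BP_Lane is an endless-runner lane that endlessly spawns pickups and obstacles at its spawn point and destroys actors reaching its killer volume.
; GetSpawnData derives delays from a drifting rolling average that trends shorter, with occasional halving or doubling; shorter delays favour harder obstacles.
; Game speed changes drive the lane material's Speed parameter.
; Construction sets lane color and keeps one initial lane, moving PlayerStart to it.
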(event OnComponentBeginOverlap(ObstacleKiller)
  (params (OverlappedComponent :type Primitive%20Component%20Object%20Reference) (OtherActor :type Actor%20Object%20Reference) (OtherComp :type Primitive%20Component%20Object%20Reference) (OtherBodyIndex :type Integer) (bFromSweep :type Boolean) (SweepResult :type Hit%20Result%20Structure%20%28by%20ref%29))
  (Actor|DestroyActor OtherActor))

(event Custom|OnGameSpeedChanged_Event_0
  (params (SelfGameMode :type BP%20Runner%20Game%20Mode%20Object%20Reference))
  (Rendering|Material|SetScalarParameterValue (Variables|Default|GetDynMatInst) "Speed" (* 3 (Variables|/Script/RunnerTest.RunnerTest_GameModeBase|GetGameSpeed SelfGameMode)) :!class /Script/Engine.MaterialInstanceDynamic))

(event EventBeginPlay
  (bind (__delay __movable) (CallFunction|GetSpawnData))
  (bind _asbp_runner_game_mode (Utilities|Casting|CastToBP_RunnerGameMode (Game|GetGameMode)))
  (bind _output_get (Variables|Default|SetRunnerGM _asbp_runner_game_mode))
  (EventDispatchers|AssignOnGameSpeedChanged _output_get (delegate Custom|OnGameSpeedChanged_Event_0))
  (bind _output_get_2 (Variables|Default|SetInitialVal (Math|Random|RandomFloatinRange 4.0 7.0)))
  (Utilities|Array|Add (Variables|Default|GetDelayArray) _output_get_2)
  (Utilities|FlowControl|Delay __delay :!label _label)
  (Game|SpawnActorfromClass __movable (Transformation|GetWorldTransform (Variables|Default|GetSpawnPoint)) "Undefined" 0 0)
  (goto _label))

(fn ConstructionScript
  (bind _staticmeshcomponent (Variables|Debug|GetStaticMeshComponent))
  (Utilities|FlowControl|Sequence
    (:then_0
      (bind _returnvalue (Rendering|Material|CreateDynamicMaterialInstance _staticmeshcomponent 2 (Utilities|Array|Get(acopy) (Rendering|Material|GetMaterials _staticmeshcomponent) 2) "None" :!class /Script/Engine.PrimitiveComponent))
      (bind _output_get (Variables|Default|SetDynMatInst _returnvalue))
      (Rendering|Material|SetVectorParameterValue _output_get "Color" (Variables|Default|GetColor) :!class /Script/Engine.MaterialInstanceDynamic))
    (:then_1
      (if (Variables|Default|GetIsInitialLane)
        (bind _outactors (Actor|GetAllActorsOfClass "BP_Lane_C"))
        (for _array_element _outactors
          (if (!= _array_element self)
            (Variables|BP_Lane_C|SetIsInitialLane _array_element false)))
        (bind _returnvalue_2 (Actor|GetActorOfClass "/Script/Engine.PlayerStart"))
        (Transformation|SetActorLocation _returnvalue_2 (Transformation|GetWorldLocation (Variables|Default|GetStartPoint)) false false)))))

(fn GetSpawnData
  (bind _returnvalue (Math|Random|RandomBoolwithWeight 0.1))
  (bind _delayarray (Variables|Default|GetDelayArray))
  (bind _delayarray_2 (Variables|Default|GetDelayArray))
  (Utilities|FlowControl|Sequence
    (:then_0
      (for _array_element _delayarray
        (LocalVariables|SetTempVal (+ (LocalVariables|GetTempVal) _array_element)))
      (bind _output_get (LocalVariables|SetTempVal (/ (LocalVariables|GetTempVal) (Math|Conversions|ToFloat(Integer) (Utilities|Array|Length _delayarray)))))
      (Utilities|Array|Add _delayarray_2 (Math|Random|RandomFloatinRange (* _output_get 0.9) (* _output_get 1.05)))
      (if (> (Utilities|Array|Length _delayarray_2) 5)
        (Utilities|Array|RemoveIndex _delayarray_2)
        (if _returnvalue
          (LocalVariables|SetTempVal (/ (LocalVariables|GetTempVal) 2.0))
          (elif _returnvalue
            (LocalVariables|SetTempVal (* (LocalVariables|GetTempVal) 2.0))
            (else
              (LocalVariables|SetTempVal (Utilities|Array|Get(acopy) _delayarray_2 (Utilities|Array|LastIndex _delayarray_2))))))))
    (:then_1
      (bind _output_get_2 (LocalVariables|SetNewLocalVar_0 (select (Math|Random|RandomBoolwithWeight 0.11) (Variables|Default|GetPickups) (select (Math|Random|RandomBoolwithWeight (Math|Float|Clamp(Float) (/ (LocalVariables|GetTempVal) (Variables|Default|GetInitialVal)))) (Variables|Default|GetEasyArray) (select (Math|Random|RandomBoolwithWeight (Math|Float|Clamp(Float) (/ (/ (LocalVariables|GetTempVal) (Variables|Default|GetInitialVal)) 2.0))) (Variables|Default|GetMediumArray) (Variables|Default|GetHardArray))))))
      (return (LocalVariables|GetTempVal) (Utilities|Array|Get(acopy) _output_get_2 (Math|Random|RandomIntegerinRange 0 (- (Utilities|Array|Length _output_get_2) 1)))))))