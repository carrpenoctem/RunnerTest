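; BP_Obstacle_Hard_1 is an endless runner obstacle that rotates its mesh while firing projectiles.
; On BeginPlay, a timeline drives a rotator lerp that turns MeshComp through nearly a full revolution.
; In parallel, a self-repeating delay loop periodically spawns BP_Projectile at StaticMesh1's location, passing MeshComp's current forward vector as its velocity.
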(event EventBeginPlay
  (|CallParentFunction)
  (Utilities|FlowControl|Sequence
    (:then_0
      (bind _newtrack_0 (Timeline|Timeline_0 PlayFromStart)
        (:Update
          (Transformation|SetRelativeRotation (Variables|Default|GetMeshComp) (Math|Rotator|Lerp(Rotator) "0, 0,0.000000" "0,359.000000,0.000000" _newtrack_0) false false))))
    (:then_1
      (Utilities|FlowControl|Delay 1.5 :!label _label)
      (Game|SpawnActorfromClass "/Game/EndlessRunner/Blueprints/BP_Projectile.BP_Projectile_C" (Math|Transform|MakeTransform (Transformation|GetWorldLocation (Variables|Default|GetStaticMesh1)) "0, 0, 0" "1,1,1") "Undefined" self (Math|Vector|GetForwardVector (Variables|Default|GetMeshComp)) 0)
      (goto _label))))

(fn ConstructionScript
  (|CallParentFunction))