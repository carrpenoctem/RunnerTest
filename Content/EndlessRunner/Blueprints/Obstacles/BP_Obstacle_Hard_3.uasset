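; Hard-tier obstacle Blueprint for the endless runner that slides its mesh sideways at a fixed raised height.
; On BeginPlay it runs the parent logic, then starts a Timeline whose track drives a vector lerp of the mesh's relative location from one side to the other, with sweep enabled.
; Overlap and Tick events are disabled stubs, and construction only calls the parent.
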(event EventBeginPlay
  (|CallParentFunction)
  (bind _newtrack_0 (Timeline|Timeline_0 PlayFromStart)
    (:Update
      (Transformation|SetRelativeLocation (Variables|Default|GetMeshComp) (Math|Vector|Lerp(Vector) "0,200.000000,160.000000" "0,-200.000000,160.000000" _newtrack_0) true false))))

(event Collision|EventActorBeginOverlap
  (params (OtherActor :type Actor%20Object%20Reference))
  (|CallParentFunction OtherActor) ; This node is disabled and will not be called.\nDrag off pins to build functionality.
)

(event EventTick
  (params (DeltaSeconds :type Float%20%28single-precision%29))
  (|CallParentFunction DeltaSeconds) ; This node is disabled and will not be called.\nDrag off pins to build functionality.
)

(fn ConstructionScript
  (|CallParentFunction))