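; BP_RunnerGameMode is the game mode for an endless runner, tracking the lanes in the level and the game speed.
; On BeginPlay it collects every BP_Lane actor into Lanes and sets CurrentLane to the one flagged as the initial lane.
; ChangeGameSpeed stores the new GameSpeed and fires the OnGameSpeedChanged dispatcher so listeners can react.
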(event Custom|ChangeGameSpeed
  (params (NewSpeed :type Float%20%28single-precision%29))
  (Variables|Default|SetGameSpeed NewSpeed)
  (Default|CallOnGameSpeedChanged self))

(event EventBeginPlay
  (Utilities|FlowControl|Sequence
    (:then_0
      (bind _outactors (Actor|GetAllActorsOfClass "/Game/EndlessRunner/Blueprints/BP_Lane.BP_Lane_C"))
      (for _array_element _outactors
        (Utilities|Array|AddUnique (Variables|Default|GetLanes) _array_element)
        (if (Variables|/Game/EndlessRunner/Blueprints/BP_Lane.BP_Lane_C|GetIsInitialLane _array_element)
          (Variables|Default|SetCurrentLane _array_element))))))

(fn ConstructionScript)